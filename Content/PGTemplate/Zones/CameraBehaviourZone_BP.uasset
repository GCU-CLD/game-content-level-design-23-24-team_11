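; Trigger zone that swaps the player camera's behaviour while the player's pawn is inside it.
; On overlap by the first player's pawn, it saves PG_PlayerCameraManager's current behaviour and applies NewCameraBehaviour.
; When that pawn leaves, it restores the saved behaviour.
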(event EventBeginPlay)

(event Collision|EventActorBeginOverlap
  (params (OtherActor :type Actor%20Object%20Reference))
  (bind _returnvalue (Game|GetPlayerController 0))
  (if (== OtherActor (Pawn|GetControlledPawn _returnvalue))
    (bind _aspg_player_camera_manager (Utilities|Casting|CastToPG_PlayerCameraManager (Variables|/Script/Engine.PlayerController|GetPlayerCameraManager _returnvalue)))
    (Variables|Default|SetOldCameraBehaviour (Variables|/Game/PGTemplate/Player/PG_PlayerCameraManager.PG_PlayerCameraManager_C|GetCurrentCameraBehaviour _aspg_player_camera_manager))
    (Variables|/Game/PGTemplate/Player/PG_PlayerCameraManager.PG_PlayerCameraManager_C|SetCurrentCameraBehaviour _aspg_player_camera_manager (Variables|Default|GetNewCameraBehaviour))))

(event EventTick
  (params (DeltaSeconds :type Float%20%28single-precision%29)))

(event Collision|EventActorEndOverlap
  (params (OtherActor :type Actor%20Object%20Reference))
  (bind _returnvalue (Game|GetPlayerController 0))
  (if (== OtherActor (Pawn|GetControlledPawn _returnvalue))
    (bind _aspg_player_camera_manager (Utilities|Casting|CastToPG_PlayerCameraManager (Variables|/Script/Engine.PlayerController|GetPlayerCameraManager _returnvalue)))
    (Variables|/Game/PGTemplate/Player/PG_PlayerCameraManager.PG_PlayerCameraManager_C|SetCurrentCameraBehaviour _aspg_player_camera_manager (Variables|Default|GetOldCameraBehaviour))))

(fn ConstructionScript)